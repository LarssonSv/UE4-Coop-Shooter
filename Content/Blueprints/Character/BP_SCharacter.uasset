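; BP_SCharacter is a character Blueprint that arms the player with a launcher weapon and shows a crosshair.
; On BeginPlay it spawns BP_Launcher with itself as owner, stores it as CurrentWeapon and snaps it to the mesh's WeaponSocket, then adds WBP_Crosshair to the viewport.
; A left mouse button key event calls Fire on CurrentWeapon directly.
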(event `self.ReceiveBeginPlay`
  (bind _returnvalue (`|SpawnActorFromClass` "/Game/Blueprints/BP_Launcher.BP_Launcher_C" (`KismetMathLibrary.MakeTransform` (0.0 0.0 0.0)) "AlwaysSpawn" "OverrideRootScale" self null))
  (set `self.CurrentWeapon` _returnvalue)
  (`self.K2_AttachToComponent` _returnvalue (`self.Mesh`) "WeaponSocket" "SnapToTarget" "SnapToTarget" "SnapToTarget" true)
  (bind _returnvalue_2 (`|CreateWidget` "/Game/UI/WBP_Crosshair.WBP_Crosshair_C"))
  (`UserWidget.AddToViewport` _returnvalue_2 0))

(event `Key|LeftMouseButton`
  (params (Key :type "Key Structure"))
  (:`Pressed`
    (`SWeapon.Fire` (`self.CurrentWeapon`))))

(fn `UserConstructionScript`)